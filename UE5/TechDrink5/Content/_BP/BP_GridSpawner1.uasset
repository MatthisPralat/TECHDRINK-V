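; BP_GridSpawner1 previews a grid layout in the editor and replaces it with physics element actors when an installation starts.
; The construction script uses a 2D grid macro to add scaled preview meshes on the local YZ plane, with exposed mesh and material.
; StartInstallation spawns BP_PhysXElem1 or BP_PhysXElem2, chosen by ModeA, at each preview transform, passes along the 3DCursor, then destroys the previews.
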(event `StartInstallation`
  (params (`3DCursor` :type "/Game/_BP/BP_3DCursor1 Object Reference"))
  (bind _3dcursor (`self.3DCursor`))
  (set `self.3DCursor` `3DCursor`)
  (for _array_element (`self.PreviewMeshes`)
    (if (`self.ModeA?`)
      (bind _returnvalue (`SceneComponent.K2_GetComponentToWorld` _array_element))
      (`|SpawnActorFromClass` "/Game/_BP/BP_PhysXElem1.BP_PhysXElem1_C" _returnvalue "Undefined" "MultiplyWithRoot" null _3dcursor null)
      (else
        (`|SpawnActorFromClass` "/Game/_BP/BP_PhysXElem2.BP_PhysXElem2_C" _returnvalue "Undefined" "MultiplyWithRoot" null _3dcursor null))))
  (for _array_element_2 (`self.PreviewMeshes`)
    (`ActorComponent.K2_DestroyComponent` _array_element_2)))

(fn `UserConstructionScript`
  ;[0 0 0 0.5 16] You have to clear the array at the start in Construction because it doesn't reset and will build up references forever until it crashes.
  (`KismetArrayLibrary.Array_Clear` (`self.PreviewMeshes`))
  (bind (_current_point _total_points _0_1_phase _poly_center) (`/Engine/ArtTools/RenderToTexture/Macros/RenderToTextureMacros.2D Grid Execution Macro` (`self.SectorSize`) (0.0 0.0 0.0) (`self.X_Amount`) (`self.Y_Amount`))
    (:`Per Poly Execution`
      (bind _returnvalue (`AddComponent|NODE_AddStaticMeshComponent-0` :`RelativeTransform` (`KismetMathLibrary.MakeTransform` (* (`KismetMathLibrary.MakeVector` 0.0 (.x _poly_center) (.y _poly_center)) (`self.CellScaling`)) (struct) (`self.MeshScale`))))
      ;[0 0 0 0.5] Add static meshes for preview and save to array to use on Begin Play. Then set Static Mesh and/or Material based on exposed parameters.
      (`KismetArrayLibrary.Array_Add` (`self.PreviewMeshes`) _returnvalue)
      (`StaticMeshComponent.SetStaticMesh` _returnvalue (`self.PreviewMesh`))
      (`PrimitiveComponent.SetMaterial` _returnvalue 0 (`self.PreviewMaterial`)))))