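; Body-tracking interface for an interactive installation, previewing sensor-tracked pelvis and hands and handling keyboard controls.
; Each tick scales OSC receiver positions onto preview meshes; keys nudge their origin offset, loaded from JSON in the user directory.
; Space hides previews, spawns the 3D cursor, starts the GridSpawner and saves the offset.
; Other keys toggle mouse/Kinect mode and pause, switch maps, quit and run display commands.
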(event `self.ReceiveBeginPlay`
  ;[0 0 0 0.5] Load JSON file on start and load the saved parameter and set to Tracking Offset.
  (bind (_outjsonobject _returnvalue) (`JsonBlueprintFunctionLibrary.FromFile` (`self.MakeJsonDir` "S2P3_Config.json")))
  (set `self.JsonObj` _outjsonobject)
  (`KismetSystemLibrary.PrintString` (`KismetStringLibrary.Conv_BoolToString` _returnvalue))
  (bind _outvalue (`|GetJsonField` (`self.JsonObj`) "TrackingOffset"))
  (bind _output_get (set `self.TrackingOffset` _outvalue))
  (`SceneComponent.K2_SetRelativeLocation` (`self.Origin`) _output_get false false))

(event `self.ReceiveTick`
  (params (DeltaSeconds :type "Float (single-precision)"))
  ;[0 0 0 0.5] Get tracking values from OSC Receiver and sale the -1 to 1 value to proper UE scale (100x or more) and apply to relative position of preview meshes.
  (`|ExecutionSequence`
    (:`then_0`
      (set `self.s_pelvis` (* (`/Game/_BP/BP_OSCReciever1.pelvis` (`self.OSC_Reciever`)) (`self.TrackingScale`)))
      (set `self.s_hand_l` (* (`/Game/_BP/BP_OSCReciever1.hand_l` (`self.OSC_Reciever`)) (`self.TrackingScale`)))
      (set `self.s_hand_r` (* (`/Game/_BP/BP_OSCReciever1.hand_r` (`self.OSC_Reciever`)) (`self.TrackingScale`)))
      (set `self.Active?` (`/Game/_BP/BP_OSCReciever1.SensorActive?` (`self.OSC_Reciever`))))
    (:`then_1`
      (`SceneComponent.K2_SetRelativeLocation` (`self.pelvis`) (`self.s_pelvis`) false false)
      (`SceneComponent.K2_SetRelativeLocation` (`self.p_hand_l`) (`self.s_hand_l`) false false)
      (`SceneComponent.K2_SetRelativeLocation` (`self.p_hand_r`) (`self.s_hand_r`) false false)
      (if (`self.Active?`)
        _))))

(event `Key|SpaceBar` :consume false
  (params (Key :type "Key Structure"))
  ;[0 0 0 0.5] Press SpaceBar to remove Preview Body Tracking Meshes, spawn 3D Cursor to begin interactivity, spawn the physics elements via GridSpawner and save offset values to JSON file.
  (:`Pressed`
    (`|ExecutionSequence`
      (:`then_0`
        (`SceneComponent.SetVisibility` (`self.p_hand_r`) false false)
        (`SceneComponent.SetVisibility` (`self.pelvis`) false false)
        (`SceneComponent.SetVisibility` (`self.p_hand_l`) false false)
        (bind _returnvalue (`|SpawnActorFromClass` "/Game/_BP/BP_3DCursor1.BP_3DCursor1_C" (`KismetMathLibrary.MakeTransform` (0.0 0.0 0.0)) "Undefined" "MultiplyWithRoot" null (`self.ModeA?`) (`self.BodyTrackMode?`) (`self.HandR?`) (`self.PreviewCursorEnabled?`) self (`self.TraceDirection`) (`self.TraceDistance`) null))
        (`/Game/_BP/BP_GridSpawner1.StartInstallation` (`self.GridSpawner`) _returnvalue))
      (:`then_1`
        (`|SetJsonField` (`self.JsonObj`) "TrackingOffset" (`self.TrackingOffset`))
        (`JsonBlueprintFunctionLibrary.ToFile` (`self.JsonObj`) (`self.MakeJsonDir` "S2P3_Config.json"))))))

(event `Key|W` :consume false
  (params (Key :type "Key Structure"))
  ;[0 0 0 0.5] Adjust & Reset Position Offset for Sensor Origin
  (:`Pressed`
    (`SceneComponent.K2_AddRelativeLocation` (`self.Origin`) (0.0 0.0 25.0) false false)
    (set `self.TrackingOffset` (`SceneComponent.RelativeLocation` (`self.Origin`)) :!label _label)))

(event `Key|S` :consume false
  (params (Key :type "Key Structure"))
  ;[0 0 0 0.5] Adjust & Reset Position Offset for Sensor Origin
  (:`Pressed`
    (`SceneComponent.K2_AddRelativeLocation` (`self.Origin`) (0.0 0.0 -25.0) false false)
    (goto _label)))

(event `Key|A` :consume false
  (params (Key :type "Key Structure"))
  ;[0 0 0 0.5] Adjust & Reset Position Offset for Sensor Origin
  (:`Pressed`
    (`SceneComponent.K2_AddRelativeLocation` (`self.Origin`) (25.0 0.0 0.0) false false)
    (goto _label)))

(event `Key|D` :consume false
  (params (Key :type "Key Structure"))
  ;[0 0 0 0.5] Adjust & Reset Position Offset for Sensor Origin
  (:`Pressed`
    (`SceneComponent.K2_AddRelativeLocation` (`self.Origin`) (-25.0 0.0 0.0) false false)
    (goto _label)))

(event `Key|Q` :consume false
  (params (Key :type "Key Structure"))
  ;[0 0 0 0.5] Adjust & Reset Position Offset for Sensor Origin
  (:`Pressed`
    (set `self.TrackingOffset` (0.0 0.0 0.0))
    (`SceneComponent.K2_SetRelativeLocation` (`self.Origin`) (0.0 0.0 0.0) false false)))

(event `Key|Escape` :consume false
  (params (Key :type "Key Structure"))
  ;[0 0 0 0.5] Packaged Game Keyboard Inputs
  (:`Pressed`
    (`KismetSystemLibrary.QuitGame` null "Quit")))

(event `Key|One` :consume false
  (params (Key :type "Key Structure"))
  ;[0 0 0 0.5] Packaged Game Keyboard Inputs
  (:`Pressed`
    (`GameplayStatics.OpenLevel` "MAP1")))

(event `Key|E` :consume false
  (params (Key :type "Key Structure"))
  ;[0 0 0 0.5] Packaged Game Keyboard Inputs
  (:`Pressed`
    (`/Engine/EditorBlueprintResources/StandardMacros.FlipFlop`
      (:`A`
        (set `self.BodyTrackMode?` false)
        (`KismetSystemLibrary.PrintString` "Input: Mouse"))
      (:`B`
        (set `self.BodyTrackMode?` true)
        (`KismetSystemLibrary.PrintString` "Input: Kinect")))))

(event `Key|Two` :consume false
  (params (Key :type "Key Structure"))
  ;[0 0 0 0.5] Packaged Game Keyboard Inputs
  (:`Pressed`
    (`GameplayStatics.OpenLevel` "MAP2")))

(event `Key|Z` :consume false
  (params (Key :type "Key Structure"))
  ;[0 0 0 0.5] Packaged Game Keyboard Inputs
  (:`Pressed`
    (`KismetSystemLibrary.ExecuteConsoleCommand` "fullscreen" null)))

(event `Key|Eight` :consume false
  (params (Key :type "Key Structure"))
  ;[0 0 0 0.5] Packaged Game Keyboard Inputs
  (:`Pressed`
    (`KismetSystemLibrary.ExecuteConsoleCommand` "scalability 2" null)))

(event `Key|X` :consume false
  (params (Key :type "Key Structure"))
  ;[0 0 0 0.5] Packaged Game Keyboard Inputs
  (:`Pressed`
    (`KismetSystemLibrary.ExecuteConsoleCommand` "stat fps" null)))

(event `Key|Nine` :consume false
  (params (Key :type "Key Structure"))
  ;[0 0 0 0.5] Packaged Game Keyboard Inputs
  (:`Pressed`
    (`KismetSystemLibrary.ExecuteConsoleCommand` "scalability 3" null)))

(event `Key|C` :consume false :paused true
  (params (Key :type "Key Structure"))
  ;[0 0 0 0.5] Packaged Game Keyboard Inputs
  (:`Pressed`
    (`/Engine/EditorBlueprintResources/StandardMacros.FlipFlop`
      (:`A`
        (`GameplayStatics.SetGamePaused` true))
      (:`B`
        (`GameplayStatics.SetGamePaused` false)))))

(fn `AttachCursorHandL`
  (params (Cursor :type "/Game/_BP/BP_3DCursor1 Object Reference"))
  ;[0 0 0 0.5] Attach 3D Cusor BP to preview mesh of Hand L
  (`self.K2_AttachToComponent` Cursor (`self.p_hand_l`) "None" "KeepRelative" "KeepRelative" "KeepRelative" true))

(fn `AttachCursorHandR`
  (params (Cursor :type "/Game/_BP/BP_3DCursor1 Object Reference"))
  ;[0 0 0 0.5] Attach 3D Cusor BP to preview mesh of Hand R
  (`self.K2_AttachToComponent` Cursor (`self.p_hand_r`) "None" "KeepRelative" "KeepRelative" "KeepRelative" true))

(fn `MakeJsonDir`
  (params (FileName :type String :default "S2P3_Config.json"))
  (returns (FilePath :type "FilePath Structure"))
  ;[0 0 0 0.5] Make JSON file directory path to User Documents folder.
  (return (make `FilePath` (`KismetStringLibrary.Concat_StrStr` (`KismetSystemLibrary.GetPlatformUserDir`) FileName))))

(fn `UserConstructionScript`)