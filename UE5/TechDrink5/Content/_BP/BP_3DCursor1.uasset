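; 3D cursor actor, driven by mouse or by body-tracked left or right hand, that interacts with physics elements.
; Each tick it line-traces a custom object channel to move HitPoint, colouring its light by Y position.
; A timed delay loop samples movement direction, smoothed to orient HitPoint, alongside speed from position history.
; Sphere overlaps toggle forces on PhysX elements; optional Niagara helpers, uncalled here, use direction and speed.
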(event `self.ReceiveBeginPlay`
  (bind _returnvalue (`GameplayStatics.GetPlayerController` 0))
  (bind _bodytrackint (`self.BodyTrackInt`))
  ;[0 0 0 0.5] Start Custom event tick with custom interval rate.
  (set `self.UpdateRate` (/ 1.0 30.0))
  (`self.CalcDir`)
  (`|ExecutionSequence`
    (:`then_0`
      ;[0 0 0 0.5] Attach itself to the preview meshes either Left or Right.
      (if (`self.HandR?`)
        (`/Game/_BP/BP_BodyTrackInterface1.AttachCursorHandR` _bodytrackint self)
        (else
          (`/Game/_BP/BP_BodyTrackInterface1.AttachCursorHandL` _bodytrackint self))))
    (:`then_1`
      ;[0 0 0 0.5] Based on exposed paramter for input mode, show or unshow cursor.
      (if (`self.BodyTrackMode?`)
        (set `PlayerController.bShowMouseCursor` false _returnvalue)
        (else
          (set `PlayerController.bShowMouseCursor` true _returnvalue))))))

(event `CalcDir`
  ;[0 0 0 0.5] Custom Event Tick loop, calculating the vector with position delta between old position and current position.
  (set `self.OldPos` (`SceneComponent.K2_GetComponentLocation` (`self.HitPoint`)))
  (`KismetSystemLibrary.Delay` (`self.UpdateRate`))
  (set `self.RawDir` (`KismetMathLibrary.Normal` (- (`SceneComponent.K2_GetComponentLocation` (`self.HitPoint`)) (`self.OldPos`)) 0.01))
  (`self.CalcDir`))

(event `self.ReceiveTick`
  (params (DeltaSeconds :type "Float (single-precision)"))
  (bind (_start _end) (`self.TraceStartEndKinect`))
  (bind (_start_2 _end_2) (`self.TraceStartEndMouse`))
  (bind (_start_3 _end_3) (`self.SelectTraceMode` _start _end _start_2 _end_2))
  (bind (_returnvalue_x _returnvalue_y) (`KismetMathLibrary.BreakVector` (`SceneComponent.K2_GetComponentLocation` (`self.HitPoint`))))
  (set `self.DeltaSec` DeltaSeconds)
  (`|ExecutionSequence`
    (:`then_0`
      ;[0 0 0 0.5] Basic Line Trace for Objects but only on 'TraceHit' custom Collision Channel with 2 input modes mouse or body tracking.
      (bind (_outhit _returnvalue) (`KismetSystemLibrary.LineTraceSingleForObjects` _start_3 _end_3 (`|MakeArray` "ObjectTypeQuery7" :!type "EObjectTypeQuery Enum")))
      (if _returnvalue
        (`SceneComponent.K2_SetWorldLocation` (`self.HitPoint`) (`.Location` (`GameplayStatics.BreakHitResult` _outhit)) false false)
        ;[0 0 0 0.5] If Preview Sphere is enabled in exposed parameter, scale based on trace hit true Scale 1,1,1 or false Scale 0,0,0
        (`self.PreviewSphereEnabled`
          (:`true`
            (`/Engine/EditorBlueprintResources/StandardMacros.DoOnce` false :!label _label
              (:`Completed`
                (`SceneComponent.SetRelativeScale3D` (`self.HitPoint`) (1.0 1.0 1.0))))))
        (else
          (`self.PreviewSphereEnabled`
            (:`true`
              (`SceneComponent.SetRelativeScale3D` (`self.HitPoint`) (0.0 0.0 0.0))
              (goto _label :!via `Reset`))))))
    (:`then_1`
      ;[0 0 0 0.5] Calculate movement velocity float with build in function and take raw movement direction and smooth it with VInterp to. Then set the Arrow component's Rotation.
      (bind _returnvalue_2 (`KismetAnimationLibrary.K2_CalculateVelocityFromPositionHistory` (`self.DeltaSec`) (`SceneComponent.K2_GetComponentLocation` (`self.HitPoint`)) (make `PositionHistory`) 30 "0.f" 1024.0))
      (set `self.CursorSpeed` _returnvalue_2)
      (bind _output_get (set `self.SmoothDir` (`KismetMathLibrary.VInterpTo` (`self.SmoothDir`) (`self.RawDir`) (`self.DeltaSec`) 12.0)))
      (`SceneComponent.K2_SetWorldRotation` (`self.HitPoint`) (`KismetMathLibrary.MakeRotFromX` _output_get) false false))
    (:`then_2`
      ;[0 0 0 0.5] Set Light Color based on Y position of Hit Point, interpolating between -250 to 250. This can be changed if your Grid is larger.
      (`LightComponent.SetLightColor` (`self.PointLight`) (`KismetMathLibrary.LinearColorLerp` (struct :`R` 1.0 :`G` 0.079394 :`A` 1.0) (struct :`G` 0.261936 :`B` 1.0 :`A` 1.0) (`KismetMathLibrary.MapRangeClamped` _returnvalue_y -250.0 250.0 0.0 1.0)) true))))

(event `self.SphereOverlap.OnComponentBeginOverlap`
  (params (OverlappedComponent :type "PrimitiveComponent Object Reference") (OtherActor :type "Actor Object Reference") (OtherComp :type "PrimitiveComponent Object Reference") (OtherBodyIndex :type Integer) (bFromSweep :type Boolean) (SweepResult :type "HitResult Structure (by ref)"))
  ;[0 0 0 0.5] Enable cursor forces application on begin-overlap and disable on end-overlap.
  (if (`self.ModeA?`)
    (bind _asbp_phys_xelem_1 (cast `/Game/_BP/BP_PhysXElem1` OtherActor))
    (`/Game/_BP/BP_PhysXElem1.SetForceEnabled` _asbp_phys_xelem_1 true)
    (else
      (bind _asbp_phys_xelem_2 (cast `/Game/_BP/BP_PhysXElem2` OtherActor))
      (`/Game/_BP/BP_PhysXElem2.SetForceEnabled` _asbp_phys_xelem_2 true))))

(event `self.SphereOverlap.OnComponentEndOverlap`
  (params (OverlappedComponent :type "PrimitiveComponent Object Reference") (OtherActor :type "Actor Object Reference") (OtherComp :type "PrimitiveComponent Object Reference") (OtherBodyIndex :type Integer))
  ;[0 0 0 0.5] Enable cursor forces application on begin-overlap and disable on end-overlap.
  (if (`self.ModeA?`)
    (bind _asbp_phys_xelem_1 (cast `/Game/_BP/BP_PhysXElem1` OtherActor))
    (`/Game/_BP/BP_PhysXElem1.SetForceEnabled` _asbp_phys_xelem_1 false)
    (else
      (bind _asbp_phys_xelem_2 (cast `/Game/_BP/BP_PhysXElem2` OtherActor))
      (`/Game/_BP/BP_PhysXElem2.SetForceEnabled` _asbp_phys_xelem_2 false))))

(fn `NiagaraDemoSpawn`
  (params (`Enabled?` :type Boolean))
  (if `Enabled?`
    (bind _returnvalue (`NiagaraFunctionLibrary.SpawnSystemAttached` "/Game/_FX/NS_CursorDemo1.NS_CursorDemo1" (`self.HitPoint`) "None" (0.0 0.0 0.0) (struct) "KeepRelativeOffset"))
    (set `self.NiagaraSystem1` _returnvalue)))

(fn `NiagaraDemoUpdate`
  (params (`Enabled?` :type Boolean))
  (bind _niagarasystem1 (`self.NiagaraSystem1`))
  (if `Enabled?`
    (`/Engine/EditorBlueprintResources/StandardMacros.IsValid` _niagarasystem1
      (:`Is Valid`
        (`NiagaraComponent.SetVariableVec3` _niagarasystem1 "Vector_Force" (* (`self.SmoothDir`) (* (`self.CursorSpeed`) 1000.0)))))))

(fn `SelectTraceMode`
  (params (Start_K :type "Vector Structure") (End_K :type "Vector Structure") (Start_M :type "Vector Structure") (End_M :type "Vector Structure"))
  (returns (Start :type "Vector Structure") (End :type "Vector Structure"))
  (bind _bodytrackmode_ (`self.BodyTrackMode?`))
  (return (select `bool` _bodytrackmode_ :`false` Start_M :`true` Start_K) (select `bool` _bodytrackmode_ :`false` End_M :`true` End_K)))

(fn `TraceStartEndKinect`
  (returns (Start :type "Vector Structure") (End :type "Vector Structure"))
  (bind _returnvalue (`self.K2_GetActorLocation`))
  ;[0 0 0 0.5] Calculate start and end point for Line Tracking for Body Tracking.
  (return _returnvalue (+ _returnvalue (* (`self.TraceDirection`) (`self.TraceDistance`)))))

(fn `TraceStartEndMouse`
  (returns (Start :type "Vector Structure") (End :type "Vector Structure"))
  (bind (_worldlocation _worlddirection) (`PlayerController.DeprojectMousePositionToWorld` (`GameplayStatics.GetPlayerController` 0)))
  ;[0 0 0 0.5] Use built in function to get mouse facing direction and scale with Trace Distance and add to get end.
  (return _worldlocation (+ _worldlocation (* _worlddirection (`self.TraceDistance`)))))

(fn `UserConstructionScript`
  (`SceneComponent.SetVisibility` (`self.HitPoint`) (`self.PreviewSphereEnabled?`) false))