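; Physics-driven element that gets pushed by the 3D cursor and glows according to how fast it moves.
; While the cursor enables force, Tick applies an impulse at ForcePoint along the cursor arrow's right vector, scaled by cursor speed.
; A dynamic material takes emissive strength from position-history velocity and an orange-to-blue color from the cursor hit point's Y.
; BeginPlay sets its UV offset from spawn Y and Z.
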(event `self.ReceiveBeginPlay`
  (bind _returnvalue (`PrimitiveComponent.CreateDynamicMaterialInstance` (`self.PC_Moving`) 0 "/Game/_MAT/M_PhysXElem3.M_PhysXElem3" "None"))
  (set `self.MAT` _returnvalue)
  ;[0 0 0 0.5 16] When messing with Actor's position in Event Tick, generally recommended to save it's initial spawn location on begin play.
  (set `self.SpawnLocation` (`self.K2_GetActorLocation`))
  ;[0 0 0 0.5 16] Generate UV Offset value based on Actor's Y and Z position and set in Material.
  (`MaterialInstanceDynamic.SetScalarParameterValue` (`self.MAT`) "UVOffset" (`self.MakeUVOffset`)))

(event `self.ReceiveTick`
  (params (DeltaSeconds :type "Float (single-precision)"))
  (bind _3dcursor (`self.3DCursor`))
  (set `self.DeltaSec` DeltaSeconds)
  (`|ExecutionSequence`
    (:`then_0`
      ;[0 0 0 0.5 16] This is set (enabled/disabled) by 3D Cursor BP using Overlap Sphere Volume
      (if (`self.ForceEnabled?`)
        (`PrimitiveComponent.AddImpulseAtLocation` (`self.PC_Moving`) (* (`SceneComponent.GetRightVector` (`/Game/_BP/BP_3DCursor1.Arrow` _3dcursor)) (* (`/Game/_BP/BP_3DCursor1.CursorSpeed` _3dcursor) 400.0)) (`SceneComponent.K2_GetComponentLocation` (`self.ForcePoint`)) "None")))
    (:`then_1`
      (bind _returnvalue (`KismetAnimationLibrary.K2_CalculateVelocityFromPositionHistory` (`self.DeltaSec`) (`SceneComponent.K2_GetComponentLocation` (`self.ForcePoint`)) (make `PositionHistory`) 15 4.0 64.0))
      (`MaterialInstanceDynamic.SetScalarParameterValue` (`self.MAT`) "EmissiveStrength" _returnvalue)
      (`MaterialInstanceDynamic.SetVectorParameterValue` (`self.MAT`) "EmissiveColor" (`self.MakeColor`)))))

(fn `MakeColor`
  (returns (Color :type "LinearColor Structure"))
  (bind (_returnvalue_x _returnvalue_y) (`KismetMathLibrary.BreakVector` (`SceneComponent.K2_GetComponentLocation` (`/Game/_BP/BP_3DCursor1.HitPoint` (`self.3DCursor`)))))
  (return (`KismetMathLibrary.LinearColorLerp` (struct :`R` 1.0 :`G` 0.079394 :`A` 1.0) (struct :`G` 0.261936 :`B` 1.0 :`A` 1.0) (`KismetMathLibrary.MapRangeClamped` _returnvalue_y -250.0 250.0 0.0 1.0))))

(fn `MakeUVOffset`
  (returns (Offset :type "Float (double-precision)"))
  (bind (_spawnlocation_x _spawnlocation_y _spawnlocation_z) (`KismetMathLibrary.BreakVector` (`self.SpawnLocation`)))
  (return (+ (`KismetMathLibrary.MapRangeClamped` _spawnlocation_y -250.0 250.0 0.0 1.0) (`KismetMathLibrary.MapRangeClamped` _spawnlocation_z 0.0 500.0 0.0 1.0))))

(fn `SetForceEnabled`
  (params (`Enabled?` :type Boolean))
  (set `self.ForceEnabled?` `Enabled?`))

(fn `UserConstructionScript`)