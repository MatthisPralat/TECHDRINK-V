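; OSC receiver Blueprint that takes body-tracking data for pelvis, left hand and right hand from an external sender.
; On BeginPlay it starts an OSC server on a hardcoded IP and port and binds a message handler.
; Each message's address is parsed as joint:axis through GetValueXYZ to build the three position vectors, swapping Y and Z.
; An "id" message sets SensorActive when its value is positive.
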(event `self.ReceiveBeginPlay`
  (bind _returnvalue (`OSCManager.CreateOSCServer` " 10.10.10.182" 3000 false true "" null))
  (bind _output_get (set `self.OSC_Server` _returnvalue))
  (add `OSCServer.OnOscMessageReceived` _output_get (`|CreateDelegate` :!event `OSC_IN`)))

(event `OSC_IN`
  (params (Message :type "OSCMessage Structure (by ref)") (IPAddress :type String) (Port :type Integer))
  (bind _output_get (set `self.OSC_MSG` Message))
  (bind _returnvalue (`OSCManager.GetOSCMessageAddress` _output_get))
  (bind _returnvalue_2 (`OSCManager.GetOSCAddressFullPath` _returnvalue))
  (set `self.OSC_Address` (`.RightS` (`KismetStringLibrary.Split` (`KismetStringLibrary.RightChop` _returnvalue_2 1) "/")))
  (`|ExecutionSequence`
    (:`then_0`
      (bind _value (`self.GetValueXYZ` "pelvis" "tx"))
      (bind _value_2 (`self.GetValueXYZ` "pelvis" "ty"))
      (bind _value_3 (`self.GetValueXYZ` "pelvis" "tz"))
      (set `self.pelvis` (`KismetMathLibrary.MakeVector` _value _value_3 _value_2)))
    (:`then_1`
      (bind _value_4 (`self.GetValueXYZ` "hand_l" "tx"))
      (bind _value_5 (`self.GetValueXYZ` "hand_l" "ty"))
      (bind _value_6 (`self.GetValueXYZ` "hand_l" "tz"))
      (set `self.hand_l` (`KismetMathLibrary.MakeVector` _value_4 _value_6 _value_5)))
    (:`then_2`
      (bind _value_7 (`self.GetValueXYZ` "hand_r" "tx"))
      (bind _value_8 (`self.GetValueXYZ` "hand_r" "ty"))
      (bind _value_9 (`self.GetValueXYZ` "hand_r" "tz"))
      (set `self.hand_r` (`KismetMathLibrary.MakeVector` _value_7 _value_9 _value_8)))
    (:`then_3`
      (if (== (`self.OSC_Address`) "id")
        (bind _value_10 (`OSCManager.GetFloat` (`self.OSC_MSG`)))
        (if (> _value_10 0.0)
          (set `self.SensorActive?` true)
          (else
            (set `self.SensorActive?` false)))))))

(fn `GetValueXYZ`
  (params (Type :type String) (Axis :type String))
  (returns (Value :type "Float (single-precision)"))
  (bind (_lefts _rights) (`KismetStringLibrary.Split` (`self.OSC_Address`) ":"))
  (if (== Type _lefts)
    (if (== Axis _rights)
      (bind _value (`OSCManager.GetFloat` (`self.OSC_MSG`)))
      (return _value))))

(fn `UserConstructionScript`)